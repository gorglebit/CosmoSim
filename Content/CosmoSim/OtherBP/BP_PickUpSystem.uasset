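; Pickup system that, on BeginPlay, spawns a grid of actors of a configurable class as a flat ring around the world origin.
; Nested length and width loops call AsteroidTransformation, which spreads instances around the Z axis and across the ring's width, adding random-stream position jitter.
; Rotation blends from ring-aligned toward random by RotationRandom, while scale is the width index times ScaleMinimumRandom, making the first index zero-sized.
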(event `self.ReceiveBeginPlay`
  (bind _instancecountbylenght (`self.InstanceCountByLenght`))
  (bind _instancecountbywidth (`self.InstanceCountByWidth`))
  (`|ExecutionSequence`
    (:`then_1`
      (for _index (range _instancecountbylenght)
        (for _index_2 (range _instancecountbywidth)
          (bind (_outlocation _outroraring) (`self.AsteroidTransformation` _index_2 _instancecountbywidth _index _instancecountbylenght))
          (`|SpawnActorFromClass` (`self.Class`) (`KismetMathLibrary.MakeTransform` _outlocation _outroraring (`KismetMathLibrary.Conv_DoubleToVector` (* _index_2 (`self.ScaleMinimumRandom`)))) "Undefined" "OverrideRootScale" null null))))))

(fn `AsteroidTransformation`
  (params (IndexFromWidthLoop :type Integer) (NumberOfInstancesByWidth :type Integer) (IndexFromLengthLoop :type Integer) (NumberOfInstancesByLength :type Integer))
  (returns (OutLocation :type "Vector Structure") (OutRoraring :type "Rotator Structure"))
  (bind _returnvalue (`KismetMathLibrary.MakeVector` 0.0 0.0 1.0))
  (bind _transformrandom (`self.TransformRandom`))
  (bind _returnvalue_2 (`KismetMathLibrary.RotateAngleAxis` (+ (+ (* (- (`KismetMathLibrary.RandomFloatFromStream` _transformrandom) 0.5) (`self.PositionZRandom`) (`self.RingWidth`)) (* (`KismetMathLibrary.RandomUnitVectorFromStream` _transformrandom) (`self.RandomizePosition`))) (`KismetMathLibrary.MakeVector` 0.0 (+ (* (- (/ (`KismetMathLibrary.Conv_IntToDouble` IndexFromWidthLoop) (`KismetMathLibrary.Conv_IntToDouble` NumberOfInstancesByWidth)) 0.5) (`self.RingWidth`)) (`self.RingRadius`)))) (* (/ (`KismetMathLibrary.Conv_IntToDouble` IndexFromLengthLoop) (`KismetMathLibrary.Conv_IntToDouble` NumberOfInstancesByLength)) 360.0) _returnvalue))
  (return _returnvalue_2 (`KismetMathLibrary.RLerp` (`KismetMathLibrary.MakeRotFromYZ` (`KismetMathLibrary.Cross_VectorVector` _returnvalue _returnvalue_2) _returnvalue) (`KismetMathLibrary.RandomRotatorFromStream` true (`self.TransformRandom`)) (`self.RotationRandom`) true)))

(fn `UserConstructionScript`)