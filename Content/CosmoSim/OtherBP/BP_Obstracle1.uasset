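; BP_Obstracle1 is a moving obstacle that triggers a hit on the player character.
; On BeginPlay, a Timeline lerps the actor from its start location 5000 units along world X without sweeping, and its Finished output calls a custom event that reverses it.
; When the Cube component hits a BP_MainCharacter, it calls that character's Hit.
; The Cube rotation logic is disconnected and never runs.
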(event `self.ReceiveBeginPlay`
  (bind _output_get (set `self.CurLoc` (`self.K2_GetActorLocation` self)))
  (set `self.Target` (+ _output_get (5000.0 0.0 0.0)))
  (bind (_direction _newtrack_0) (`Timeline|Timeline_0` :!label _label)
    (:`Update`
      (`self.K2_SetActorLocation` self (`KismetMathLibrary.VLerp` (`self.CurLoc`) (`self.Target`) _newtrack_0) false false))
    (:`Finished`
      (`self.CustomEvent_0`))))

(event `self.ReceiveTick`
  (params (DeltaSeconds :type "Float (single-precision)")))

(event `CustomEvent_0`
  (goto _label :!via `Reverse`))

(event `self.Cube.OnComponentHit`
  (params (HitComponent :type "PrimitiveComponent Object Reference") (OtherActor :type "Actor Object Reference") (OtherComp :type "PrimitiveComponent Object Reference") (NormalImpulse :type "Vector Structure") (Hit :type "HitResult Structure (by ref)"))
  (bind _asbp_main_character (cast `/Game/CosmoSim/Character/BP_MainCharacter` OtherActor))
  (`/Game/CosmoSim/Character/BP_MainCharacter.Hit` _asbp_main_character))

(fn `UserConstructionScript`)