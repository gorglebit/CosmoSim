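; BP_MenuCharacter is a menu actor that animates the main camera between a menu view and a start view.
; On BeginPlay it stores the world transforms of MainCamera and CameraStart as the two endpoints.
; A single timeline lerps MainCamera between them, playing forward for MoveCameratoStart and reversing for Movecameratomenu to return to the menu view.
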(event `self.ReceiveBeginPlay`
  (set `self.Start` (`SceneComponent.K2_GetComponentToWorld` (`self.CameraStart`)))
  (set `self.Menu` (`SceneComponent.K2_GetComponentToWorld` (`self.MainCamera`))))

(event `Move Camera to Start`
  (bind (_direction _newtrack_0) (`Timeline|Timeline_0` :!label _label)
    (:`Update`
      (`SceneComponent.K2_SetWorldTransform` (`self.MainCamera`) (`KismetMathLibrary.TLerp` (`self.Menu`) (`self.Start`) _newtrack_0) false false))))

(event `Move camera to menu`
  (goto _label :!via `Reverse`))

(event `self.ReceiveTick`
  (params (DeltaSeconds :type "Float (single-precision)")))

(fn `UserConstructionScript`)