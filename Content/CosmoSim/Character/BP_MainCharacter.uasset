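; Main player character that drops into a physics ragdoll on the R key or a Hit event and stands back up on the U key or GetUp event.
; While ragdolled, Tick moves the capsule to the pelvis and line traces from it to choose the front or back get-up montage.
; Standing up plays that montage, stops physics, reattaches the mesh to the capsule and briefly disables input.
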(event `self.ReceiveTick`
  (params (DeltaSeconds :type "Float (single-precision)"))
  (bind _returnvalue (`SceneComponent.GetSocketLocation` (`self.Mesh`) "pelvis"))
  (`|ExecutionSequence`
    (:`then_0`)
    (:`then_1`
      ;[1 1 1] Set Get Up AM
      (if (`self.IsRagdollOn`)
        (`SceneComponent.K2_SetWorldLocation` (`self.CapsuleComponent`) _returnvalue false false)
        (bind (_outhit _returnvalue_2) (`KismetSystemLibrary.LineTraceSingle` _returnvalue (+ _returnvalue (* (`KismetMathLibrary.GetRightVector` (`SceneComponent.GetSocketRotation` (`self.Mesh`) "pelves")) (50.0 50.0 50.0))) "TraceTypeQuery1"))
        (if _returnvalue_2
          (set `self.StandUpMontage` "/Game/CosmoSim/Character/Anim/GroundLocomotion/AM_GetUpFront.AM_GetUpFront")
          (else
            (set `self.StandUpMontage` "/Game/CosmoSim/Character/Anim/GroundLocomotion/AM_GetUpBack.AM_GetUpBack")))))))

(event `Key|R`
  (params (Key :type "Key Structure"))
  (bind _mesh (`self.Mesh`))
  ;[1 1 1] Ragdoll
  (:`Pressed`
    (set `self.IsRagdollOn` true :!label _label)
    (`PrimitiveComponent.SetSimulatePhysics` _mesh true)
    (`PrimitiveComponent.SetCollisionProfileName` _mesh "Ragdoll" true)))

(event `Hit`
  ;[1 1 1] Ragdoll
  (goto _label))

(event `Key|U`
  (params (Key :type "Key Structure"))
  ;[1 1 1] StandUp
  (:`Pressed`
    (if (`self.IsRagdollOn`) :!label _label_2
      (`self.DisableInput` (`GameplayStatics.GetPlayerController` 0))
      (`|PlayMontage` (`self.Mesh`) (`self.StandUpMontage`)
        (:`then`
          (`PrimitiveComponent.SetSimulatePhysics` (`self.Mesh`) false)
          (set `self.IsRagdollOn` false)
          (`SceneComponent.K2_AttachToComponent` (`self.Mesh`) (`self.CapsuleComponent`) "None" "KeepRelative" "KeepRelative" "KeepRelative" true)
          (`SceneComponent.K2_SetRelativeLocationAndRotation` (`self.Mesh`) (0.0 0.0 -90.0) (struct :`Yaw` 270.0) false false)
          (`KismetSystemLibrary.Delay` 2.0)
          (`self.EnableInput` (`GameplayStatics.GetPlayerController` 0)))))))

(event `GetUp`
  ;[1 1 1] StandUp
  (goto _label_2))

(fn `UserConstructionScript`)